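; Boss ground attack actor whose box collision grows over time and then removes itself.
; Tick captures the starting scale once, then lerps BoxCollisionSize toward a hardcoded scale over Duration, resetting the timer when Duration elapses.
; The actor destroys itself once the lerped scale is within a small distance of the TargetScale variable, which is separate from the hardcoded lerp end.
; Box overlap only prints a debug string; no damage is applied here.
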(event `self.ReceiveBeginPlay`)

(event `self.ReceiveTick`
  (params (DeltaSeconds :type "Float (single-precision)"))
  (bind _boxcollisionsize (`self.BoxCollisionSize`))
  (bind _returnvalue (`KismetMathLibrary.VLerp` (`self.StartScale`) (20.0 5.0 3.0) (/ (`self.ElapsedTime`) (`self.Duration`))))
  ;[1 1 1] 보스 GroundAttack 콜리전 사이즈 변화
  ;;[1 1 1] 초기사이즈 경과 시간에 따라 누적
  (bind _output_get (set `self.ElapsedTime` (+ (`self.ElapsedTime`) (`GameplayStatics.GetWorldDeltaSeconds`))))
  (if (not (`self.bInit`))
    (set `self.bInit` true)
    (set `self.StartScale` (`SceneComponent.K2_GetComponentScale` _boxcollisionsize)))
  (if (>= _output_get (`self.Duration`))
    (set `self.ElapsedTime` 0.0)
    (else
      ;;[1 1 1] Lerp로 사이즈 점차 증가
      (`SceneComponent.SetWorldScale3D` _boxcollisionsize _returnvalue)
      ;[1 1 1] 사이즈가 원하는만큼 변화되면 삭제
      (if (<= (`KismetMathLibrary.VSize` (- (`self.TargetScale`) _returnvalue)) 0.5)
        (`self.K2_DestroyActor`)))))

(event `self.Box.OnComponentBeginOverlap`
  (params (OverlappedComponent :type "PrimitiveComponent Object Reference") (OtherActor :type "Actor Object Reference") (OtherComp :type "PrimitiveComponent Object Reference") (OtherBodyIndex :type Integer) (bFromSweep :type Boolean) (SweepResult :type "HitResult Structure (by ref)"))
  (`KismetSystemLibrary.PrintString` "Hello"))

(fn `UserConstructionScript`)