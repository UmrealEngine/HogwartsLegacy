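; BP_BossSpawnLight is an actor that produces a temporary light effect, apparently for a boss spawn, then removes itself.
; On BeginPlay a timeline ramps the intensity of its Re light component up from zero.
; Tick watches for near-peak intensity and starts a second timeline that lerps from the current intensity toward zero, compounding the fade each update.
; The actor destroys itself once that value reaches zero.
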(event `self.ReceiveBeginPlay`
  (bind (_direction _bossspawn) (`Timeline|Timeline` :`NewTime` 3.0)
    (:`Update`
      (`LightComponent.SetIntensity` (`self.re`) (`KismetMathLibrary.Lerp` 0.0 5000.0 _bossspawn)))))

(event `self.ReceiveTick`
  (params (DeltaSeconds :type "Float (single-precision)"))
  (bind _intensity (`LightComponentBase.Intensity` (`self.re`)))
  (if (> _intensity 4900.0)
    (bind (_direction _bossspawn) (`Timeline|Timeline_0` :`NewTime` 3.0)
      (:`Update`
        (bind _returnvalue (`KismetMathLibrary.Lerp` _intensity 0.0 _bossspawn))
        (`LightComponent.SetIntensity` (`self.re`) _returnvalue)
        (if (<= _returnvalue 0.0)
          (`self.K2_DestroyActor`))))))

(fn `UserConstructionScript`)