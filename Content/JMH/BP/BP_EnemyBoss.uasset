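; Boss enemy that turns to face the player, attacks on timers, updates an HP widget when damaged and plays a death montage.
; Tick periodically fires an energy ball from a socket on a montage notify, paused while the ground skill is active.
; The ground skill lerps box collision scale over time, then resets it; its montage branch is unreachable.
; UpdateState and DamageState are never called here, and TransitionState is empty.
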(event `self.ReceiveBeginPlay`
  ;[1 1 1] HP UI
  (set `self.GroundSkillInitScale` (`SceneComponent.K2_GetComponentScale` (`self.BoxCollisionSize`)))
  (bind _output_get (set `self.HP` (`self.MaxHP`)))
  (bind _aswbp_boss_hp (cast `/Game/JMH/UI/WBP_BossHP` (`WidgetComponent.GetWidget` (`self.HPW`))))
  (bind _output_get_2 (set `self.WBBossHP` _aswbp_boss_hp))
  (`/Game/JMH/UI/WBP_BossHP.UpdateHPUI` _output_get_2 _output_get (`self.MaxHP`)))

(event `self.ReceiveAnyDamage`
  (params (Damage :type "Float (single-precision)") (DamageType :type "DamageType Object Reference") (InstigatedBy :type "Controller Object Reference") (DamageCauser :type "Actor Object Reference"))
  ;[1 1 1] Damage
  (if (not (`self.bdeath`))
    (bind _output_get (set `self.HP` (`KismetMathLibrary.FClamp` (- (`self.HP`) Damage) 0.0 (`self.MaxHP`))))
    (`/Game/JMH/UI/WBP_BossHP.UpdateHPUI` (`self.WBBossHP`) _output_get (`self.MaxHP`))
    (if (<= (`self.HP`) 0.0)
      (`self.Death`))))

(event `Death`
  ;[1 1 1] Death
  (set `self.bdeath` true)
  (`|PlayMontage` (`self.Mesh`) "/Game/JMH/Anim/Boss/anim2/Boss_Die_Montage.Boss_Die_Montage"
    (:`then`
      (`KismetSystemLibrary.Delay` 100.0))))

(event `self.ReceiveTick`
  (params (DeltaSeconds :type "Float (single-precision)"))
  (bind _mesh (`self.Mesh`))
  (bind _groundskilltime (`self.GroundSkillTime`))
  (if (not (`self.bdeath`))
    (`self.LookAtRotation`)
    (`|ExecutionSequence`
      (:`then_0`
        (`KismetSystemLibrary.PrintString` (`KismetStringLibrary.Conv_DoubleToString` _groundskilltime) true true (struct :`G` 0.66 :`B` 1.0 :`A` 1.0) 5.0 "-1")
        (bind _output_get (set `self.GroundSkillTime` (+ _groundskilltime DeltaSeconds)))
        (if (>= _output_get 10.0)
          (bind _output_get_2 (set `self.bGroundSkillPlay` true))
          (if (not _output_get_2)
            ;[1 1 1] Ground Skill
            (`|PlayMontage` (`self.Mesh`) "/Game/JMH/Anim/Boss/anim2/Boss_GroundSkill_Montage.Boss_GroundSkill_Montage"
              (:`OnNotifyBegin`
                _)))
          (`self.BossGroundSkill`)))
      (:`then_1`
        (bind _output_get_3 (set `self.EnergySkillTime` (+ (`self.EnergySkillTime`) DeltaSeconds)))
        (if (>= _output_get_3 4.0)
          (if (not (`self.bGroundSkillPlay`))
            (set `self.EnergySkillTime` 0.0)
            ;[1 1 1] Energy
            (`|PlayMontage` (`self.Mesh`) "/Game/JMH/Anim/Boss/anim2/Boss_EnergySkillB_Montage.Boss_EnergySkillB_Montage"
              (:`OnNotifyBegin`
                (`|SpawnActorFromClass` "/Game/JMH/BP/BP_Projectile_BossEnergyBall.BP_Projectile_BossEnergyBall_C" (`KismetMathLibrary.MakeTransform` (`SceneComponent.GetSocketLocation` _mesh "BossSocket") (`SceneComponent.GetSocketRotation` _mesh "BossSocket")) "AlwaysSpawn" "MultiplyWithRoot" null 1200.0 0.0 null)
                (set `self.EnergySkillTime` 0.0)))))))))

(event `self.CapsuleComponent.OnComponentBeginOverlap`
  (params (OverlappedComponent :type "PrimitiveComponent Object Reference") (OtherActor :type "Actor Object Reference") (OtherComp :type "PrimitiveComponent Object Reference") (OtherBodyIndex :type Integer) (bFromSweep :type Boolean) (SweepResult :type "HitResult Structure (by ref)")))

(event `LookAtRotation`
  (bind (_returnvalue_x _returnvalue_y) (`KismetMathLibrary.BreakVector` (`self.K2_GetActorLocation`)))
  (bind _returnvalue (`GameplayStatics.GetPlayerCharacter` 0))
  (bind (_returnvalue_x_2 _returnvalue_y_2) (`KismetMathLibrary.BreakVector` (`self.K2_GetActorLocation` _returnvalue)))
  (bind (_returnvalue_x_3 _returnvalue_y_3) (`KismetMathLibrary.BreakVector` (- (`KismetMathLibrary.MakeVector` _returnvalue_x_2 _returnvalue_y_2) (`KismetMathLibrary.MakeVector` _returnvalue_x _returnvalue_y))))
  ;[1 1 1] 플레이어 방향으로 회전
  (`/Engine/EditorBlueprintResources/StandardMacros.IsValid` _returnvalue
    (:`Is Valid`
      (`self.K2_SetActorRotation` (`KismetMathLibrary.MakeRotFromX` (`KismetMathLibrary.MakeVector` _returnvalue_x_3 _returnvalue_y_3))))))

(fn `BossGroundSkill`
  (`self.InterpolateSize`))

(fn `DamageState`
  (params (DamageAmount :type "Float (double-precision)"))
  (set `self.HP` (- (`self.HP`) DamageAmount))
  (if (<= (`self.HP`) 0.0)
    (`self.Death`)))

(fn `InterpolateSize`
  (bind _targetscale_x (`KismetMathLibrary.BreakVector` (`self.TargetScale`)))
  (bind _boxcollisionsize (`self.BoxCollisionSize`))
  (bind _returnvalue (`KismetMathLibrary.VLerp` (`self.StartScale`) (3.0 3.0 3.0) (/ (`self.ElapsedTime`) (`self.Duration`))))
  ;[1 1 1] 보스 GroundAttack 콜리전 사이즈 변화
  ;;[1 1 1] 초기사이즈 경과 시간에 따라 누적
  (bind _output_get (set `self.ElapsedTime` (+ (`self.ElapsedTime`) (`GameplayStatics.GetWorldDeltaSeconds`))))
  (if (not (`self.bInit`))
    (set `self.bInit` true)
    (set `self.StartScale` (`SceneComponent.K2_GetComponentScale` _boxcollisionsize)))
  (if (>= _output_get (`self.Duration`))
    (set `self.ElapsedTime` 0.0)
    (else
      ;;[1 1 1] Lerp로 사이즈 점차 증가
      (`SceneComponent.SetWorldScale3D` _boxcollisionsize _returnvalue)
      (bind _output_get_2 (set `self.LerpVector` _returnvalue))
      ;[1 1 1] 사이즈가 원하는만큼 변화되면 초기화
      (if (<= (- (.x _output_get_2) _targetscale_x) 0.1)
        (set `self.GroundSkillTime` 0.0)
        (set `self.bGroundSkillPlay` false)
        (`SceneComponent.SetWorldScale3D` (`self.BoxCollisionSize`) (`self.GroundSkillInitScale`))
        (else
          (`KismetSystemLibrary.PrintString` "Hello"))))))

(fn `Play Montage`
  (params (Montage :type "AnimMontage Object Reference"))
  (`self.Play Montage` Montage)
  (return))

(fn `TransitionState`)

(fn `UpdateState`
  (switch `/Game/JMH/BP/E_EnemyState` (`self.currentState`)
    (:`NewEnumerator3`
      (`self.DamageState` 0.0))
    (:`NewEnumerator4`
      (`self.LookAtRotation`))
    (:`NewEnumerator6`
      (`self.BossGroundSkill`))))

(fn `UserConstructionScript`)