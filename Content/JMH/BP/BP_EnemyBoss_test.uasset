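; Boss enemy that opens with a camera-blend and shake intro, then attacks the player until killed and brings up the clear screen.
; Looping timers fire energy-ball and ground skills, spawning their actors from montage notifies, with flags suppressing hit reactions and overlapping energy casts.
; Tick turns it toward the player on yaw and swaps overlay outline materials by target state.
; Lethal damage stops the timers, kills Knight2 enemies and plays death.
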(event `self.ReceiveAnyDamage`
  (params (Damage :type "Float (single-precision)") (DamageType :type "DamageType Object Reference") (InstigatedBy :type "Controller Object Reference") (DamageCauser :type "Actor Object Reference"))
  (bind _returnvalue (- (`self.HP`) Damage))
  ;[1 1 1] Damage
  (if (not (`self.bIsDead`))
    (if (`self.bSpawn`)
      (if (> _returnvalue 0.0)
        (set `self.HP` (`KismetMathLibrary.FClamp` _returnvalue 0.0 (`self.MaxHP`)) :!label _label)
        (if (not (`self.bSkill`))
          (`self.PlayAnimMontage` "/Game/JMH/Anim/Boss02/Standing_UE_Anim_Montage.Standing_UE_Anim_Montage"))
        (elif (<= _returnvalue 0.0)
          (set `self.HP` 0.0)
          (`self.StopAnimMontage` null)
          (`/Engine/EditorBlueprintResources/StandardMacros.DoOnce` false
            (:`Completed`
              (set `self.bIsDead` true)
              (`self.Death`)))
          (else
            (goto _label)))))))

(event `self.ReceiveBeginPlay`
  ;[1 1 1] HP UI
  (bind _output_get (set `self.HP` (`self.MaxHP`)))
  (bind _returnvalue (`|CreateWidget` "/Game/JMH/UI/WBP_BossHP.WBP_BossHP_C"))
  (bind _output_get_2 (set `self.WBBossHP` _returnvalue))
  (`/Game/JMH/UI/WBP_BossHP.UpdateHPUI` _output_get_2 _output_get (`self.MaxHP`) "")
  (bind _asbp_player (cast `/Game/Suhyeok/BP_Player` (`GameplayStatics.GetPlayerPawn` 0)))
  (bind _output_get_3 (set `self.Player` _asbp_player))
  (`self.DisableInput` _output_get_3 null)
  ;[1 1 1] BossCamera
  (bind _outactors (`GameplayStatics.GetAllActorsWithTag` "BossCamera"))
  (`PlayerController.SetViewTargetWithBlend` (`GameplayStatics.GetPlayerController` 0) (`|GetArrayItem` _outactors) 0.5 "VTBlend_Linear" 0.0 false)
  (`GameplayStatics.PlayWorldCameraShake` "/Game/JMH/BP/BP_CameraShake_Boss.BP_CameraShake_Boss_C" (`self.K2_GetActorLocation`) 0.0 1000.0)
  (set `self.bSpawn` true)
  (`self.SwitchToPlayerCamera`)
  (`self.EnableInput` (`self.Player`) null)
  (`KismetSystemLibrary.Delay` 0.2)
  ;[1 1 1] Damage
  (`self.EnergySkill`)
  (bind _returnvalue_2 (`KismetSystemLibrary.K2_SetTimerDelegate` (delegate `EnergySkill`) 5.0 true))
  (bind _returnvalue_3 (`KismetSystemLibrary.K2_SetTimerDelegate` (delegate `GroundSkill`) 15.0 true)))

(event `Death`
  ;[1 1 1] Death
  (set `self.bIsDead` true)
  (`KismetSystemLibrary.K2_ClearAndInvalidateTimerHandle` (stale `self.ReceiveBeginPlay` _returnvalue_2))
  (`KismetSystemLibrary.K2_ClearAndInvalidateTimerHandle` (stale `self.ReceiveBeginPlay` _returnvalue_3))
  (`GameplayStatics.PlayWorldCameraShake` "/Game/JMH/BP/BP_CameraShake_Boss.BP_CameraShake_Boss_C" (`self.K2_GetActorLocation`))
  (`self.Enemy kill`)
  (`self.StopAnimMontage` null)
  (`|PlayMontage` (`self.Mesh`) "/Game/JMH/Anim/Boss02/REBoss_Die_Montage.REBoss_Die_Montage"
    (:`then`
      _)
    (:`OnCompleted`
      _))
  (`WidgetLayoutLibrary.RemoveAllWidgets`)
  (`KismetSystemLibrary.Delay` 6.0)
  (bind _returnvalue (`|CreateWidget` "/Game/JMH/UI/WBP_Clear.WBP_Clear_C"))
  (`UserWidget.AddToViewport` _returnvalue 0))

(event `Enemy kill`
  (bind _outactors (`GameplayStatics.GetAllActorsOfClass` "/Game/SeungWoo/Enemies/BP_Enemy_Knight2.BP_Enemy_Knight2_C"))
  (`/Game/SeungWoo/Enemies/BP_Enemy_Knight2.Death` _outactors))

(event `SwitchToPlayerCamera`
  (`PlayerController.SetViewTargetWithBlend` (`GameplayStatics.GetPlayerController` 0) (`GameplayStatics.GetPlayerCharacter` 0) 0.5 "VTBlend_Linear" 0.0 false))

(event `GroundSkill`
  ;[1 1 1] Ground Skill
  (if (not (`self.bIsDead`))
    (set `self.bSkill` true)
    (set `self.bSkillPlaytoggle` true)
    (if (`self.bSkillPlaytoggle`)
      (`GameplayStatics.PlayWorldCameraShake` "/Game/JMH/BP/BP_CameraShake_Boss.BP_CameraShake_Boss_C" (`self.K2_GetActorLocation`) 0.0 1000.0)
      (`|PlayMontage` (`self.Mesh`) "/Game/JMH/Anim/Boss02/REBoss_GroundSkill_Montage.REBoss_GroundSkill_Montage"
        (:`OnCompleted`
          (set `self.bSkillPlaytoggle` false)
          (set `self.bSkill` false))
        (:`OnNotifyBegin`
          (`|SpawnActorFromClass` "/Game/JMH/BP/BP_BossGroundSkill.BP_BossGroundSkill_C" (`KismetMathLibrary.MakeTransform` (`self.K2_GetActorLocation`) (`KismetMathLibrary.Conv_VectorToRotator` (`self.GetActorForwardVector`))) "AlwaysSpawn" "MultiplyWithRoot" null null))))))

(event `EnergySkill`
  (bind _mesh (`self.Mesh`))
  ;[1 1 1] Energy
  (if (not (`self.bIsDead`))
    (set `self.bSkill` true)
    (if (not (`self.bSkillPlaytoggle`))
      (`KismetSystemLibrary.Delay` 2.0)
      (`|PlayMontage` (`self.Mesh`) "/Game/JMH/Anim/Boss02/REBoss_EnergySkillB_Montage.REBoss_EnergySkillB_Montage"
        (:`OnNotifyBegin`
          (`|SpawnActorFromClass` "/Game/JMH/BP/BP_Projectile_BossEnergyBall.BP_Projectile_BossEnergyBall_C" (`KismetMathLibrary.MakeTransform` (`SceneComponent.GetSocketLocation` _mesh "BossSocket") (`SceneComponent.GetSocketRotation` _mesh "BossSocket")) "AlwaysSpawn" "MultiplyWithRoot" null 1800.0 0.0 null)
          (set `self.bSkill` false))))))

(event `self.ReceiveTick`
  (params (DeltaSeconds :type "Float (single-precision)"))
  (if (`self.bSpawn`)
    ;[1 1 1] OutLine
    (if (not (`self.bIsDead`))
      (`self.LookAtRotation`)
      (if (== self (`/Game/Suhyeok/BP_Player.Current Target` (`self.Player`)))
        (`MeshComponent.SetOverlayMaterial` (`self.Mesh`) "/Game/Suhyeok/UI/AutoTarget/M_OutLine.M_OutLine")
        (else
          (`MeshComponent.SetOverlayMaterial` (`self.Mesh`) "/Game/Suhyeok/UI/AutoTarget/M_OutLine2.M_OutLine2"))))))

(event `LookAtRotation`
  (bind (_returnvalue_x _returnvalue_y) (`KismetMathLibrary.BreakVector` (`self.K2_GetActorLocation`)))
  (bind _returnvalue (`GameplayStatics.GetPlayerCharacter` 0))
  (bind (_returnvalue_x_2 _returnvalue_y_2) (`KismetMathLibrary.BreakVector` (`self.K2_GetActorLocation` _returnvalue)))
  (bind (_returnvalue_x_3 _returnvalue_y_3) (`KismetMathLibrary.BreakVector` (- (`KismetMathLibrary.MakeVector` _returnvalue_x_2 _returnvalue_y_2) (`KismetMathLibrary.MakeVector` _returnvalue_x _returnvalue_y))))
  ;[1 1 1] 플레이어 방향으로 회전
  (if (not (`self.bIsDead`))
    (`/Engine/EditorBlueprintResources/StandardMacros.IsValid` _returnvalue
      (:`Is Valid`
        (`self.K2_SetActorRotation` (`KismetMathLibrary.MakeRotFromX` (`KismetMathLibrary.MakeVector` _returnvalue_x_3 _returnvalue_y_3)))))))

(event `self.CapsuleComponent.OnComponentBeginOverlap`
  (params (OverlappedComponent :type "PrimitiveComponent Object Reference") (OtherActor :type "Actor Object Reference") (OtherComp :type "PrimitiveComponent Object Reference") (OtherBodyIndex :type Integer) (bFromSweep :type Boolean) (SweepResult :type "HitResult Structure (by ref)")))

(fn `DamageState`
  (params (DamageAmount :type "Float (double-precision)"))
  (set `self.HP` (- (`self.HP`) DamageAmount))
  (if (<= (`self.HP`) 0.0)
    (`self.Death`)))

(fn `UserConstructionScript`)