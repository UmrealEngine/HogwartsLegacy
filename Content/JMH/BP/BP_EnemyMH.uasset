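; Enemy Blueprint, apparently a boss, that chases the player after its PawnSensing component spots a pawn.
; Sighting sets a flag that is never cleared and starts ChasePlayer, which repeats AI MoveTo one second after each successful move.
; A state machine is scaffolded but unfinished: UpdateState dispatches on CurrentState but is never called, and TransitionState and most state functions are empty.
; Attack only plays a boss idle montage.
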(event `self.ReceiveTick`
  (params (DeltaSeconds :type "Float (single-precision)")))

(event `ChasePlayer`
  (if (`self.IsSeeingPlayer`)
    (`|AIMoveTo` self (0.0 0.0 0.0) (`GameplayStatics.GetPlayerCharacter` 0)
      (:`then`
        (`KismetSystemLibrary.Delay` 1.0)
        (`self.ChasePlayer`)))))

(event `self.PawnSensing.OnSeePawn`
  (params (Pawn :type "Pawn Object Reference"))
  (set `self.IsSeeingPlayer` true)
  (`self.ChasePlayer`))

(event `Attack`
  (`|PlayMontage` (`self.Mesh`) "/Game/JMH/Anim/Boss/Boss_Idle_Montage.Boss_Idle_Montage"))

(fn `Chase`)

(fn `DamageState`)

(fn `Die`)

(fn `Idle`)

(fn `SkillA`)

(fn `SkillB`)

(fn `TransitionState`
  (if (`|EnumEquality` (`self.currentState`) (`self.nextState`))
    _))

(fn `UpdateState`
  (switch `/Game/JMH/BP/E_EnemyState` (`self.currentState`)
    (:`NewEnumerator2`
      (`self.Attack`))
    (:`NewEnumerator3`
      (`self.DamageState`))
    (:`NewEnumerator4`
      (`self.Die`))
    (:`NewEnumerator5`
      (`self.SkillA`))
    (:`NewEnumerator6`
      (`self.SkillB`))))

(fn `UserConstructionScript`)