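; Boss energy ball projectile Blueprint that damages the player on contact.
; When its Sphere1 component begins an overlap, it applies fixed damage only if the other actor is tagged Player.
; Any such overlap, tagged or not, spawns an impact emitter and sound at the ball's location, then destroys it.
; BeginPlay and actor overlap just call the parent; the node forcing Sphere1 as the movement's updated component is unconnected.
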(event `self.ReceiveBeginPlay`
  (`parent.ReceiveBeginPlay`))

(event `self.ReceiveActorBeginOverlap`
  (params (OtherActor :type "Actor Object Reference"))
  (`parent.ReceiveActorBeginOverlap` OtherActor))

(event `self.Sphere1.OnComponentBeginOverlap`
  (params (OverlappedComponent :type "PrimitiveComponent Object Reference") (OtherActor :type "Actor Object Reference") (OtherComp :type "PrimitiveComponent Object Reference") (OtherBodyIndex :type Integer) (bFromSweep :type Boolean) (SweepResult :type "HitResult Structure (by ref)"))
  (bind _returnvalue (`self.K2_GetActorLocation`))
  ;[1 1 1] Damage
  (if (`self.ActorHasTag` OtherActor "Player")
    (`GameplayStatics.ApplyDamage` OtherActor 10.0))
  (`GameplayStatics.SpawnEmitterAtLocation` (`self.Emitter Template`) _returnvalue)
  (`GameplayStatics.PlaySoundAtLocation` (`self.Impact Sound`) _returnvalue (struct) 1.0 1.0 0.0 null null null null)
  (`self.K2_DestroyActor`))

(fn `UserConstructionScript`
  (`parent.UserConstructionScript`))