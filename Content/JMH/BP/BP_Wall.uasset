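; BP_Wall is a targetable wall actor that blows up when hit by player-style projectiles.
; Each tick it swaps the mesh overlay material to show whether it is the player's CurrentTarget, using a player reference cached on BeginPlay.
; Overlap with a BP_BoomBullet or BP_BasicAttackBullet spawns BP_EXBoomBoxSphere, plays an explosion sound and destroys the wall.
; The force events are empty, with their physics impulse logic left disconnected.
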(event `self.ReceiveBeginPlay`
  (`self.Load Current Target OutLine`))

(event `self.ReceiveTick`
  (params (DeltaSeconds :type "Float (single-precision)"))
  (`self.Set Current Target OutLine `))

(event `self.ApplyForce`
  (params (ForceOrigin :type "Vector Structure") (Power :type "Float (double-precision)")))

(event `self.ApplyForceWithDirection`
  (params (DirectionVector :type "Vector Structure") (Power :type "Float (double-precision)") (`1` :type "Transform Structure")))

(event `self.ResetForce`)

(event `self.ReceiveActorBeginOverlap`
  (params (OtherActor :type "Actor Object Reference"))
  ;[1 1 1] BoomBullet 오버랩 시 폭탄
  (bind _output_get (set `self.OverlapActor` OtherActor))
  (cast `/Game/Suhyeok/Skill/Boom/BP_BoomBullet` _output_get
    (:`then`
      _)
    (:`CastFailed`
      (cast `/Game/Suhyeok/Skill/BasicAttack/BP_BasicAttackBullet` _output_get)))
  (bind _returnvalue (`|SpawnActorFromClass` "/Game/Suhyeok/Skill/PushPull/BP_EXBoomBoxSphere.BP_EXBoomBoxSphere_C" (`KismetMathLibrary.MakeTransform` (`SceneComponent.K2_GetComponentLocation` (`self.StaticMesh`))) "Undefined" "MultiplyWithRoot" null null))
  (`GameplayStatics.PlaySoundAtLocation` "/Game/Suhyeok/Sound/DescendoBoxBoom.DescendoBoxBoom" (`self.K2_GetActorLocation` _returnvalue) (struct) 1.0 1.0 0.0 null null null null)
  (`self.K2_DestroyActor`))

(fn `Load Current Target OutLine`
  (bind _asbp_player (cast `/Game/Suhyeok/BP_Player` (`GameplayStatics.GetPlayerPawn` 0)))
  (set `self.PlayerCurrentTarget` _asbp_player))

(fn `Set Current Target OutLine `
  (if (== self (`/Game/Suhyeok/BP_Player.Current Target` (`self.PlayerCurrentTarget`)))
    (`MeshComponent.SetOverlayMaterial` (`self.StaticMesh`) "/Game/Suhyeok/UI/AutoTarget/M_OutLine.M_OutLine")
    (else
      (`MeshComponent.SetOverlayMaterial` (`self.StaticMesh`) "/Game/Suhyeok/UI/AutoTarget/M_OutLine2.M_OutLine2"))))

(fn `UserConstructionScript`)