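; BP_Enemy_Base is a base enemy that chases the player and plays a zombie attack animation on reaching them.
; On BeginPlay it runs AI MoveTo toward the player character; on success it plays the attack montage and restarts the chase after a short delay.
; The loop continues only through the success branch, so a failed move ends the chase.
; The attack is animation only, with no damage logic in this graph.
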(event `self.ReceiveBeginPlay`
  (`self.ChasePlayer`))

(event `ChasePlayer`
  (`|AIMoveTo` self (0.0 0.0 0.0) (`GameplayStatics.GetPlayerCharacter` 0) 150.0
    (:`OnSuccess`
      (`self.Attack`)
      (`KismetSystemLibrary.Delay` 0.2)
      (`self.ChasePlayer`))))

(event `Attack`
  (`|PlayMontage` (`self.Mesh`) "/Game/Characters/Mannequins/Animations/Manny/zombieattack_UE_Montage.zombieattack_UE_Montage"))

(fn `UserConstructionScript`)