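; Knight enemy Blueprint that chases the player and attacks with a greatsword slash.
; ChasePlayer moves to the player, calls Attack and repeats after a fixed delay, but stops looping if the move fails.
; Attack plays the slash montage and fires OnAttackEnd on completion or interruption.
; WieldSword spawns BP_Sword on the right-hand socket; BeginPlay is empty and the only call to WieldSword here is disconnected.
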(event `Chase Player`
  (`|AIMoveTo` self (0.0 0.0 0.0) (`GameplayStatics.GetPlayerCharacter` 0) 300.0
    (:`OnSuccess`
      (`self.Attack`)
      (`KismetSystemLibrary.Delay` 2.0)
      (`self.Chase Player`))))

(event `Attack`
  (`|PlayMontage` (`self.Mesh`) "/Game/SeungWoo/Animation/GreatSwordSlash_UE_Montage.GreatSwordSlash_UE_Montage"
    (:`OnCompleted`
      _)
    (:`OnInterrupted`
      _))
  (`self.OnAttackEnd`))

(event `WieldSword`
  (bind _returnvalue (`|SpawnActorFromClass` "/Game/Weapon_Pack/Blueprints/BP_Sword.BP_Sword_C" (`self.GetTransform`) "Undefined" "MultiplyWithRoot" null null))
  (`self.K2_AttachToComponent` _returnvalue (`self.Mesh`) "hand_r_sword_socket" "SnapToTarget" "SnapToTarget" "SnapToTarget" true)
  (set `self.isWieldingSword` true))

(event `self.ReceiveBeginPlay`)

(fn `UserConstructionScript`)