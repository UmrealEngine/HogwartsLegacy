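; Knight enemy that plays a stand-up montage on spawn, then chases the player with AIMoveTo, slashing on arrival and repeating.
; Box overlaps damage Player-tagged actors once per swing via an attacking flag; incoming damage reduces HP until a death montage and destroy.
; Tick swaps the overlay outline material when the knight is the player's current target.
; HP bar setup, distance-based states and manual movement are leftover, disconnected or uncalled logic.
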(event `self.ReceiveBeginPlay`
  ;[1 1 1] 스폰 애니메이션
  ;[1 1 1] Player 변수 지정
  (bind _asbp_player (cast `/Game/Suhyeok/BP_Player` (`GameplayStatics.GetPlayerPawn` 0)))
  (set `self.PlayerPawn` _asbp_player)
  (`|PlayMontage` (`self.Mesh`) "/Game/SeungWoo/Animation/Standing_UE_Montage1.Standing_UE_Montage1"
    (:`OnCompleted`
      (`self.Chase Player`))))

(event `HPdecresepersec`
  ;[1 1 1] HP 1초마다 줄어드는 디버깅용
  (bind _result (`/Engine/EditorBlueprintResources/StandardMacros.DecrementFloat` (`self.HP`))
    (:`  `
      (bind _output_get (set `self.HP` _result))
      (`KismetSystemLibrary.PrintString` (`KismetStringLibrary.Conv_DoubleToString` _output_get))
      (if (<= _output_get 0.0)
        (`self.Death`)))))

(event `self.ReceiveAnyDamage`
  (params (Damage :type "Float (single-precision)") (DamageType :type "DamageType Object Reference") (InstigatedBy :type "Controller Object Reference") (DamageCauser :type "Actor Object Reference"))
  ;[1 1 1] 데미지 받는 코드
  (if (not (`self.Bdeth`))
    (bind _output_get (set `self.HP` (`KismetMathLibrary.FClamp` (- (`self.HP`) Damage) 0.0 (`self.Max HP`))))
    (if (<= (`self.HP`) 0.0)
      (`self.Death`))))

(event `Chase Player`
  ;[1 1 1] Player 따라가다 attack 실행하는 코드
  (`|AIMoveTo` self (0.0 0.0 0.0) (`GameplayStatics.GetPlayerCharacter` 0) 150.0
    (:`OnSuccess`
      (`self.Attack`)
      (`KismetSystemLibrary.Delay` 2.0)
      (`self.Chase Player`))))

(event `WieldSword`
  ;[1 1 1] 무기 손에 생성
  (bind _returnvalue (`|SpawnActorFromClass` "/Game/Weapon_Pack/Blueprints/BP_Sword.BP_Sword_C" (`self.GetTransform`) "Undefined" "MultiplyWithRoot" null null))
  (bind _output_get (set `self.SwordActor` _returnvalue))
  (`self.K2_AttachToComponent` _output_get (`self.Mesh`) "hand_r_sword_socket" "SnapToTarget" "SnapToTarget" "SnapToTarget" true)
  (set `self.isWieldingSword` true))

(event `Attack`
  ;[1 1 1] Slash 애니메이션 몽타주 실행
  (if (not (`self.Bdeth`))
    (set `self.BIsAttacking` true)
    (`|PlayMontage` (`self.Mesh`) "/Game/SeungWoo/Animation/GreatSwordSlash_UE1_Montage.GreatSwordSlash_UE1_Montage"
      (:`OnCompleted`
        _)
      (:`OnInterrupted`
        _))
    (set `self.BIsAttacking` false)
    (`self.OnAttackEnd`)))

(event `FocusPawn`
  (bind (_returnvalue_roll _returnvalue_pitch _returnvalue_yaw) (`KismetMathLibrary.BreakRotator` (`KismetMathLibrary.FindLookAtRotation` (`self.K2_GetActorLocation`) (`self.K2_GetActorLocation` (`GameplayStatics.GetPlayerPawn` 0)))))
  ;[1 1 1] 플레이어 쪽 바라보기
  (`self.K2_SetActorRotation` (`KismetMathLibrary.MakeRotator` _returnvalue_roll 0.0 _returnvalue_yaw)))

(event `MovetoPawn`
  (params (DeltaTime :type "Float (double-precision)") (Direction :type "Vector Structure") (Speed :type "Float (double-precision)"))
  ;[1 1 1] 이동 함수: P=P0+vt
  (`self.K2_SetActorLocation` (+ (`self.K2_GetActorLocation`) (* Direction Speed DeltaTime))))

(event `Death`
  ;[1 1 1] Actor Destroy
  (set `self.Bdeth` true)
  (bind _returnvalue (`self.PlayAnimMontage` "/Game/SeungWoo/Animation/FlyingBackDeath_UE_Montage.FlyingBackDeath_UE_Montage"))
  (`KismetSystemLibrary.Delay` (/ _returnvalue 2.0))
  (`self.K2_DestroyActor`))

(event `SpeedSeting`
  (bind _charactermovement (`self.CharacterMovement`))
  ;[1 1 1] 속도 설정
  (switch `/Game/SeungWoo/Enemies/AI/Enums/E_AIState` "NewEnumerator0"
    (:`NewEnumerator0`
      (set `CharacterMovementComponent.MinAnalogWalkSpeed` 100.0 _charactermovement)
      (set `CharacterMovementComponent.MaxWalkSpeed` 100.0 _charactermovement))
    (:`NewEnumerator1`
      (set `CharacterMovementComponent.MinAnalogWalkSpeed` 500.0 _charactermovement)
      (set `CharacterMovementComponent.MaxWalkSpeed` 400.0 _charactermovement))))

(event `DistanceState`
  ;[1 1 1] 거리에 따른 상태 부여
  (if (< (`self.GetDistanceTo` (`GameplayStatics.GetPlayerPawn` 0)) 400.0)
    (set `self.State` "NewEnumerator1")
    (`KismetSystemLibrary.PrintString` "Attacking")
    (else
      (set `self.State` "NewEnumerator0")
      (`KismetSystemLibrary.PrintString` "Passive"))))

(event `self.ReceiveTick`
  (params (DeltaSeconds :type "Float (single-precision)"))
  ;[1 1 1] 아웃라이너
  (if (== self (`/Game/Suhyeok/BP_Player.Current Target` (`self.PlayerPawn`)))
    (`MeshComponent.SetOverlayMaterial` (`self.Mesh`) "/Game/Suhyeok/UI/AutoTarget/M_OutLine.M_OutLine")
    (else
      (`MeshComponent.SetOverlayMaterial` (`self.Mesh`) "/Game/Suhyeok/UI/AutoTarget/M_OutLine2.M_OutLine2"))))

(event `self.Box.OnComponentBeginOverlap`
  (params (OverlappedComponent :type "PrimitiveComponent Object Reference") (OtherActor :type "Actor Object Reference") (OtherComp :type "PrimitiveComponent Object Reference") (OtherBodyIndex :type Integer) (bFromSweep :type Boolean) (SweepResult :type "HitResult Structure (by ref)"))
  ;[1 1 1] Player에게 데미지 주기(Sword
  (if (`self.ActorHasTag` OtherActor "Player")
    (if (`self.BIsAttacking`)
      (`GameplayStatics.ApplyDamage` null 10.0)
      (set `self.BIsAttacking` false))))

(fn `GetPatrolRoute`
  (returns (PatrolRoute :type "/Game/SeungWoo/Enemies/AI/BP_PatrollRoute Object Reference"))
  (return (`self.PatrolRoute`)))

(fn `SetMovementSpeed`
  (params (Speed :type "/Game/SeungWoo/Enemies/AI/Enums/E_MovementSpeed Enum" :default "NewEnumerator0"))
  (returns (SpeedValue :type "Float (double-precision)"))
  (bind _output_get (set `CharacterMovementComponent.MaxWalkSpeed` (select `/Game/SeungWoo/Enemies/AI/Enums/E_MovementSpeed` Speed :`NewEnumerator1` 100.0 :`NewEnumerator2` 300.0 :`NewEnumerator3` 500.0 :!type "Float (single-precision)") (`self.CharacterMovement`)))
  (return _output_get))

(fn `UserConstructionScript`)