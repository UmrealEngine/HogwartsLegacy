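; Zombie enemy that turns to face the player each tick and lunges when within close range.
; Dash briefly overrides movement velocity along the forward vector, restores it, then waits out a cooldown.
; DashAttack plays the attack montage behind a DoOnce fired at BeginPlay and never reset in live logic, so it plays once.
; ChasePlayer uses AIMoveTo but is not called here; several disconnected experiments remain.
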(event `self.ReceiveBeginPlay`
  (`self.DashAttack`))

(event `ChasePlayer`
  (`|AIMoveTo` self (0.0 0.0 0.0) (`GameplayStatics.GetPlayerPawn` 0)
    (:`OnSuccess`
      (`self.DashAttack`))))

(event `DashAttack`
  (`/Engine/EditorBlueprintResources/StandardMacros.DoOnce` false
    (:`Completed`
      (`KismetSystemLibrary.PrintString` "attack")
      (bind _returnvalue (`self.PlayAnimMontage` "/Game/SeungWoo/Characters/Mannequins/Animations/Manny/zombieattack_UE_Montage.zombieattack_UE_Montage")))))

(event `self.ReceiveTick`
  (params (DeltaSeconds :type "Float (single-precision)"))
  (bind _output_get (set `self.Direction` (`KismetMathLibrary.Normal` (`KismetMathLibrary.Conv_Vector2DToVector` (`KismetMathLibrary.Conv_VectorToVector2D` (- (`self.K2_GetActorLocation` (`GameplayStatics.GetPlayerPawn` 0)) (`self.K2_GetActorLocation`)))))))
  (`self.K2_SetActorRotation` (`KismetMathLibrary.Conv_VectorToRotator` _output_get))
  (if (< (`self.GetDistanceTo` (`GameplayStatics.GetPlayerPawn` 0)) 500.0)
    (`self.Dash`)
    (`self.DashAttack`)))

(event `Dash`
  (if (`self.CanDash?`)
    (`KismetSystemLibrary.PrintString` "Dash")
    (set `self.CanDash?` false)
    (set `self.OldVelocity` (`MovementComponent.Velocity` (`self.CharacterMovement`)))
    (set `MovementComponent.Velocity` (* (`self.GetActorForwardVector`) 5000.0) (`self.CharacterMovement`))
    (`KismetSystemLibrary.Delay` 0.2)
    (set `MovementComponent.Velocity` (`self.OldVelocity`) (`self.CharacterMovement`))
    (`KismetSystemLibrary.Delay` (`self.DasCooldown`))
    (set `self.CanDash?` true)))

(fn `UserConstructionScript`)