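; BP_BasicAttackBullet is the projectile for the basic attack skill, resolving its hit on actor overlap.
; Every overlap spawns a BP_BloodExplosion_BasicAttack effect at the other actor's transform, whatever that actor is.
; Actors tagged NormalEnemy or Boss take the same fixed damage, and the bullet destroys itself in every case.
; An unconnected branch for destroying BoomBox1-tagged actors never runs.
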(event `self.ReceiveActorBeginOverlap`
  (params (OtherActor :type "Actor Object Reference"))
  (bind _overlapactor (`self.OverlapActor`))
  (bind _overlapactor_2 (`self.OverlapActor`))
  (`|SpawnActorFromClass` "/Game/Suhyeok/Skill/BasicAttack/2/BP_BloodExplosion_BasicAttack.BP_BloodExplosion_BasicAttack_C" (`self.GetTransform` OtherActor) "Undefined" "MultiplyWithRoot" null null)
  (set `self.OverlapActor` OtherActor)
  (if (`self.ActorHasTag` _overlapactor_2 "NormalEnemy")
    (`GameplayStatics.ApplyDamage` _overlapactor_2 10.0)
    (`self.K2_DestroyActor`)
    (elif (`self.ActorHasTag` _overlapactor "Boss")
      (`GameplayStatics.ApplyDamage` _overlapactor 10.0)
      (`self.K2_DestroyActor`)
      (else
        (`self.K2_DestroyActor`)))))

(fn `UserConstructionScript`)