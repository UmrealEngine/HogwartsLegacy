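; Player component that runs a three-hit basic attack combo by playing montages on the owning BP_Player's mesh.
; BasicAttack buffers a press in SaveAttack while IsAttacking, otherwise plays the attack selected by AttackIndex, each behind a DoOnce and short delay.
; BasicAttackCombo continues a buffered combo or resets it through StopCombo.
; The attack input event is empty, the CanAttack check is unwired, and IsAttacking is never set true here.
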(event `self.ReceiveBeginPlay`
  (bind _asbp_player (cast `/Game/Suhyeok/BP_Player` (`self.GetOwner`)))
  (set `self.Character Mesh` (`Character.Mesh` _asbp_player)))

(event `EnhancedInput|/Game/Suhyeok/Actions/Input/IA_PlayerAttack`
  (params (ActionValue :type Boolean) (ElapsedSeconds :type "Float (double-precision)") (TriggeredSeconds :type "Float (double-precision)") (InputAction :type "InputAction Object Reference" :default "/Game/Suhyeok/Actions/Input/IA_PlayerAttack.IA_PlayerAttack"))
  ;[0.1168 0.1168 0.1168] Attack Input
)

(event `Attack 1`
  ;[1 1 1] Attack 1
  (`/Engine/EditorBlueprintResources/StandardMacros.DoOnce` false :!label _label
    (:`Completed`
      (`KismetSystemLibrary.Delay` 0.1)
      (`|PlayMontage` (`self.Character Mesh`) "/Game/Suhyeok/Skill/BasicAttack/BasicSkillAnimation/PlayerBasicAttack01_UE_Montage.PlayerBasicAttack01_UE_Montage"
        (:`then`
          (set `self.AttackIndex` 1)
          (goto _label :!via `Reset`))))))

(event `BasicAttack`
  ;[0.2775 0.2775 0.2775] Basic Attack
  (if (`self.IsAttacking?`)
    (set `self.SaveAttack?` true)
    (else
      (set `self.SaveAttack?` false)
      (switch `int` (`self.AttackIndex`) :!label _label_2
        (:`0`
          (`self.Attack 1`))
        (:`1`
          (`self.Attack 2`))
        (:`2`
          (`self.Attack 3`))))))

(event `Attack 2`
  ;[1 1 1] Attack 2
  ;;[0.3192 0.3192 0.3192] Combo Continue
  (`/Engine/EditorBlueprintResources/StandardMacros.DoOnce` false :!label _label_3
    (:`Completed`
      (`KismetSystemLibrary.Delay` 0.1)
      (`|PlayMontage` (`self.Character Mesh`) "/Game/Suhyeok/Skill/BasicAttack/BasicSkillAnimation/PlayerBasicAttack02_UE_Montage.PlayerBasicAttack02_UE_Montage"
        (:`then`
          (set `self.AttackIndex` 2)
          (goto _label_3 :!via `Reset`))))))

(event `BasicAttackCombo`
  ;[0.3192 0.3192 0.3192] Combo Continue
  (if (`self.SaveAttack?`)
    (set `self.SaveAttack?` false)
    (goto _label_2)
    (else
      (`self.StopCombo`))))

(event `StopCombo`
  ;[0.3579 0.3579 0.3579] Stop Combo / Attack
  (set `self.IsAttacking?` false)
  (set `self.AttackIndex` 0))

(event `Attack 3`
  ;[1 1 1] Attack 3
  (`/Engine/EditorBlueprintResources/StandardMacros.DoOnce` false :!label _label_4
    (:`Completed`
      (`KismetSystemLibrary.Delay` 0.1)
      (`|PlayMontage` (`self.Character Mesh`) "/Game/Suhyeok/Skill/BasicAttack/BasicSkillAnimation/PlayerBasicAttack03_UE_Montage.PlayerBasicAttack03_UE_Montage"
        (:`then`
          (set `self.AttackIndex` 3)
          (goto _label_4 :!via `Reset`))))))