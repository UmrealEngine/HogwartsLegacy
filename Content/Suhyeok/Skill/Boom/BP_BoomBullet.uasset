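; BP_BoomBullet is a skill projectile that spawns a BP_EndBoom at the transform of any actor it overlaps, then destroys itself.
; On overlap it checks tags to apply damage, with Boss set to take double the NormalEnemy amount.
; The NormalEnemy damage call has no target actor connected, so only the Boss branch passes the overlapped actor to ApplyDamage.
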(event `self.ReceiveActorBeginOverlap`
  (params (OtherActor :type "Actor Object Reference"))
  (bind _overlapactor (`self.OverlapActor`))
  (`|SpawnActorFromClass` "/Game/Suhyeok/Skill/Boom/3/BP_EndBoom.BP_EndBoom_C" (`self.GetTransform` OtherActor) "Undefined" "MultiplyWithRoot" null null)
  (set `self.OverlapActor` OtherActor)
  (if (`self.ActorHasTag` (`self.OverlapActor`) "NormalEnemy")
    (`GameplayStatics.ApplyDamage` null 10.0)
    (`self.K2_DestroyActor`)
    (elif (`self.ActorHasTag` _overlapactor "Boss")
      (`GameplayStatics.ApplyDamage` _overlapactor 20.0)
      (`self.K2_DestroyActor`)
      (else
        (`self.K2_DestroyActor`)))))

(fn `UserConstructionScript`)