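; BP_EXBoomSmall is a small explosion skill actor that damages or destroys what it overlaps.
; Every overlap first spawns BP_EndBoom at the other actor's transform, whatever its tag.
; Tag checks then damage NormalEnemy and Boss actors, with bosses taking more, and destroy BoomBox1 actors outright.
; Damaging hits also play a BP_Camera2 world shake centered on the player pawn, and the actor never destroys itself here.
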(event `self.ReceiveActorBeginOverlap`
  (params (OtherActor :type "Actor Object Reference"))
  (bind _overlapactor (`self.OverlapActor`))
  (bind _overlapactor_2 (`self.OverlapActor`))
  (`|SpawnActorFromClass` "/Game/Suhyeok/Skill/Boom/3/BP_EndBoom.BP_EndBoom_C" (`self.GetTransform` OtherActor) "Undefined" "MultiplyWithRoot" null null)
  (set `self.OverlapActor` OtherActor)
  (if (`self.ActorHasTag` _overlapactor_2 "NormalEnemy")
    (`GameplayStatics.ApplyDamage` _overlapactor_2 30.0)
    (`GameplayStatics.PlayWorldCameraShake` "/Game/Suhyeok/Camera/BP_Camera2.BP_Camera2_C" (`self.K2_GetActorLocation` (`GameplayStatics.GetPlayerPawn` 0)) 0.0 4000.0)
    (elif (`self.ActorHasTag` (`self.OverlapActor`) "BoomBox1")
      (`self.K2_DestroyActor` (`self.OverlapActor`))
      (elif (`self.ActorHasTag` _overlapactor "Boss")
        (`GameplayStatics.ApplyDamage` _overlapactor 40.0)
        (`GameplayStatics.PlayWorldCameraShake` "/Game/Suhyeok/Camera/BP_Camera2.BP_Camera2_C" (`self.K2_GetActorLocation` (`GameplayStatics.GetPlayerPawn` 0)) 0.0 4000.0)))))

(fn `UserConstructionScript`)