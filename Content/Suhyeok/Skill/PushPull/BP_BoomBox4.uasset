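; BP_BoomBox4 is an explosive box actor that can be pushed by external forces and explodes when shot.
; Force events enable physics on the Box and apply a mass-independent impulse, either away from an origin or along a given direction.
; ResetForce stops simulation, moves the actor to the Box's location and reattaches the Box.
; Overlap with a boom or basic attack bullet spawns an explosion emitter and BP_EXBoomBoxSphere, then destroys the actor.
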(event `self.ApplyForce`
  (params (ForceOrigin :type "Vector Structure") (Power :type "Float (double-precision)"))
  (`PrimitiveComponent.SetSimulatePhysics` (`self.Box`) true)
  (`PrimitiveComponent.AddImpulse` (`self.Box`) (* (`KismetMathLibrary.Normal` (- (`SceneComponent.K2_GetComponentLocation` (`self.Box`)) ForceOrigin)) Power) "None" true))

(event `self.ApplyForceWithDirection`
  (params (DirectionVector :type "Vector Structure") (Power :type "Float (double-precision)") (`1` :type "Transform Structure"))
  (`PrimitiveComponent.SetSimulatePhysics` (`self.Box`) true)
  (`PrimitiveComponent.AddImpulse` (`self.Box`) (* DirectionVector Power) "None" true))

(event `self.ResetForce`
  (if (`SceneComponent.IsSimulatingPhysics` (`self.Box`) "None")
    (`PrimitiveComponent.SetSimulatePhysics` (`self.Box`) false)
    (`self.K2_SetActorLocation` (`SceneComponent.K2_GetComponentLocation` (`self.Box`)))
    (`SceneComponent.K2_AttachToComponent` (`self.Box`) null "None" "KeepWorld" "KeepWorld" "KeepWorld" true)))

(event `self.ReceiveActorBeginOverlap`
  (params (OtherActor :type "Actor Object Reference"))
  (bind _returnvalue (`SceneComponent.K2_GetComponentLocation` (`self.StaticMesh`)))
  ;[1 1 1] BoomBullet 오버랩 시 폭탄
  (bind _output_get (set `self.OverlapActor` OtherActor))
  (cast `/Game/Suhyeok/Skill/Boom/BP_BoomBullet` _output_get
    (:`then`
      _)
    (:`CastFailed`
      (cast `/Game/Suhyeok/Skill/BasicAttack/BP_BasicAttackBullet` _output_get)))
  (`GameplayStatics.SpawnEmitterAtLocation` "/Game/StarterContent/Particles/P_Explosion.P_Explosion" _returnvalue (struct) (4.0 4.0 4.0))
  (`|SpawnActorFromClass` "/Game/Suhyeok/Skill/PushPull/BP_EXBoomBoxSphere.BP_EXBoomBoxSphere_C" (`KismetMathLibrary.MakeTransform` _returnvalue) "Undefined" "MultiplyWithRoot" null null)
  (`self.K2_DestroyActor`))

(fn `UserConstructionScript`)