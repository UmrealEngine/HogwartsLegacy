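; BP_EXBoomBoxSphere is an overlap damage actor in the PushPull skill folder, apparently the explosion sphere for a BoomBox.
; On begin overlap it branches on the other actor's tags.
; NormalEnemy actors take damage and are immediately destroyed, BoomBox1 actors are destroyed without damage, and Boss actors take heavier damage but are not destroyed by it.
; The sphere has no logic to spawn, time or remove itself.
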(event `self.ReceiveActorBeginOverlap`
  (params (OtherActor :type "Actor Object Reference"))
  (bind _overlapactor (`self.OverlapActor`))
  (bind _overlapactor_2 (`self.OverlapActor`))
  (set `self.OverlapActor` OtherActor)
  (if (`self.ActorHasTag` _overlapactor_2 "NormalEnemy")
    (`GameplayStatics.ApplyDamage` _overlapactor_2 10.0)
    (`self.K2_DestroyActor` (`self.OverlapActor`))
    (elif (`self.ActorHasTag` (`self.OverlapActor`) "BoomBox1")
      (`self.K2_DestroyActor` (`self.OverlapActor`))
      (elif (`self.ActorHasTag` _overlapactor "Boss")
        (`GameplayStatics.ApplyDamage` _overlapactor 30.0)))))

(fn `UserConstructionScript`)