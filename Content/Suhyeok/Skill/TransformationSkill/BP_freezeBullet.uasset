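; Freeze bullet for the Transformation skill that turns a normal enemy it hits into a frozen enemy.
; On sphere overlap with an actor tagged NormalEnemy, it destroys that enemy and itself, then spawns BP_FreezeEnemy at the bullet's transform rather than the enemy's.
; It also plays a transformation sound at the new enemy and spawns a nature aura effect actor just below it.
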(event `self.ReceiveBeginPlay`)

(event `self.Sphere.OnComponentBeginOverlap`
  (params (OverlappedComponent :type "PrimitiveComponent Object Reference") (OtherActor :type "Actor Object Reference") (OtherComp :type "PrimitiveComponent Object Reference") (OtherBodyIndex :type Integer) (bFromSweep :type Boolean) (SweepResult :type "HitResult Structure (by ref)"))
  (bind _output_get (set `self.Overlap Actor` OtherActor))
  (if (`self.ActorHasTag` _output_get "NormalEnemy")
    (`self.K2_DestroyActor` _output_get)
    (`self.K2_DestroyActor`)
    (bind _returnvalue (`|SpawnActorFromClass` "/Game/Suhyeok/BP_FreezeEnemy.BP_FreezeEnemy_C" (`self.GetTransform`) "Undefined" "MultiplyWithRoot" null null))
    (bind _returnvalue_2 (`self.K2_GetActorLocation` _returnvalue))
    (`GameplayStatics.PlaySoundAtLocation` "/Game/Suhyeok/Sound/Transformation__cut_2sec_.Transformation__cut_2sec_" _returnvalue_2 (struct) 1.0 1.0 0.0 null null null null)
    (`|SpawnActorFromClass` "/Game/Suhyeok/Skill/TransformationSkill/2/BP_N_NatureAura_Transformation.BP_N_NatureAura_Transformation_C" (`KismetMathLibrary.MakeTransform` (+ _returnvalue_2 (0.0 0.0 -100.0))) "Undefined" "MultiplyWithRoot" null null)))

(fn `UserConstructionScript`)